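; StrayAsteroid is a spinning asteroid obstacle that gets knocked away when struck by TheShip or a LaserBeam.
; BeginPlay randomizes its material, X/Y scale and yaw spin rate.
; Ship or laser overlaps, and laser hits, store the impact normal as launch vector; collision turns off, though overlaps require a nonzero normal.
; Tick spins it and, once hit, moves it along that vector at a fixed per-frame step, unscaled by delta time.
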(event `self.Capsule.OnComponentBeginOverlap`
  (params (OverlappedComponent :type "PrimitiveComponent Object Reference") (OtherActor :type "Actor Object Reference") (OtherComp :type "PrimitiveComponent Object Reference") (OtherBodyIndex :type Integer) (bFromSweep :type Boolean) (SweepResult :type "HitResult Structure (by ref)"))
  (cast `/Game/Blueprints/TheShip` OtherActor
    (:`then`
      _)
    (:`CastFailed`
      (cast `/Game/Blueprints/LaserBeam` OtherActor)))
  (set `self.IsHit` true)
  (bind _output_get (set `self.SetLaunchVector` (`.ImpactNormal` (`GameplayStatics.BreakHitResult` SweepResult))))
  (if (> (`KismetMathLibrary.VSize` _output_get) 0.0)
    (`PrimitiveComponent.SetCollisionEnabled` (`self.Capsule`) "NoCollision" :!label _label)
    (`PrimitiveComponent.SetCollisionEnabled` (`self.LaserBeamMesh`) "NoCollision")))

(event `self.ReceiveActorBeginOverlap`
  (params (OtherActor :type "Actor Object Reference")))

(event `self.ReceiveBeginPlay`
  (bind _returnvalue (`KismetMathLibrary.RandomFloatInRange` 0.5 3.0))
  (`PrimitiveComponent.SetMaterial` (`self.LaserBeamMesh`) 0 (`|GetArrayItem` (`self.AsteroidMaterial`) (`KismetMathLibrary.RandomIntegerInRange` 0 2)))
  (`self.SetActorScale3D` (`KismetMathLibrary.MakeVector` _returnvalue _returnvalue 1.0))
  (set `self.RandomRotation` (`KismetMathLibrary.RandomFloatInRange` 0.5 2.0)))

(event `self.ReceiveTick`
  (params (DeltaSeconds :type "Float (single-precision)"))
  (`SceneComponent.K2_AddRelativeRotation` (`self.DefaultSceneRoot`) (`KismetMathLibrary.MakeRotator` 0.0 0.0 (`self.RandomRotation`)) false false)
  (if (`self.IsHit`)
    (`self.K2_AddActorWorldOffset` (* (`self.SetLaunchVector`) 20.0))))

(event `self.Capsule.OnComponentHit`
  (params (HitComponent :type "PrimitiveComponent Object Reference") (OtherActor :type "Actor Object Reference") (OtherComp :type "PrimitiveComponent Object Reference") (NormalImpulse :type "Vector Structure") (Hit :type "HitResult Structure (by ref)"))
  (cast `/Game/Blueprints/LaserBeam` OtherActor)
  (set `self.SetLaunchVector` (* (`.ImpactNormal` (`GameplayStatics.BreakHitResult` Hit)) 1.0))
  (set `self.IsHit` true)
  (goto _label))

(fn `UserConstructionScript`)