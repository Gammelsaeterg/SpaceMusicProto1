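; A rotating planet actor that offers dialogue to the player's ship and can reward it with a module.
; Overlap shows an interaction indicator and registers the planet as the ship's current dialogue box; leaving clears the widgets and disables interaction.
; Each ShowDialogue call displays the next widget class from TextToSpawn.
; The call after the last page closes and resets the dialogue, then optionally installs the chosen module and calls CheckShip.
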(event `self.ReceiveTick`
  (params (DeltaSeconds :type "Float (single-precision)"))
  (`SceneComponent.K2_AddRelativeRotation` (`self.ThePlanet`) (`KismetMathLibrary.MakeRotator` 0.0 0.0 (`self.RotatingSpeed`)) false false))

(event `self.ReceiveActorBeginOverlap`
  (params (OtherActor :type "Actor Object Reference"))
  (cast `/Game/Blueprints/TheShip` OtherActor)
  (bind _returnvalue (`|CreateWidget` "/Game/UI/InteractionIndicator.InteractionIndicator_C"))
  (bind _output_get (set `self.InteractionIndicator` _returnvalue))
  (`UserWidget.AddToViewport` _output_get 0)
  (bind _asthe_ship (cast `/Game/Blueprints/TheShip` OtherActor))
  (set `/Game/Blueprints/TheShip.IsAbleToInteract` true _asthe_ship)
  (set `/Game/Blueprints/TheShip.CurrentDialougeBox` (`ActorComponent.GetOwner` (`self.DefaultSceneRoot`)) _asthe_ship))

(event `self.ReceiveActorEndOverlap`
  (params (OtherActor :type "Actor Object Reference"))
  (bind _interactionindicator (`self.InteractionIndicator`))
  (bind _spawnedtext (`self.SpawnedText`))
  (cast `/Game/Blueprints/TheShip` OtherActor)
  (if (`KismetSystemLibrary.IsValid` _interactionindicator)
    (`Widget.RemoveFromParent` _interactionindicator))
  (if (`KismetSystemLibrary.IsValid` _spawnedtext)
    (`Widget.RemoveFromParent` _spawnedtext))
  (bind _asthe_ship (cast `/Game/Blueprints/TheShip` OtherActor))
  (set `/Game/Blueprints/TheShip.IsAbleToInteract` false _asthe_ship))

(fn `ShowDialogue`
  (bind _spawnedtext (`self.SpawnedText`))
  (bind _spawnedtext_2 (`self.SpawnedText`))
  (if (`self.NoMoreText`)
    (if (`KismetSystemLibrary.IsValid` _spawnedtext_2)
      (`Widget.RemoveFromParent` _spawnedtext_2))
    (set `self.CurrentIndex` 0)
    (set `self.NoMoreText` false)
    (`UserWidget.AddToViewport` (`self.InteractionIndicator`) 0)
    (if (`self.GiveModule?`)
      (bind _asthe_ship (cast `/Game/Blueprints/TheShip` (`GameplayStatics.GetPlayerPawn` 0)))
      (`KismetArrayLibrary.Array_Set` (`/Game/Blueprints/TheShip.ModulesInstalled` _asthe_ship) (`self.WhichModule`) true)
      (`/Game/Blueprints/TheShip.CheckShip` _asthe_ship))
    (else
      (`Widget.RemoveFromParent` (`self.InteractionIndicator`))
      (if (`KismetSystemLibrary.IsValid` _spawnedtext)
        (`Widget.RemoveFromParent` _spawnedtext))
      (bind _returnvalue (`|CreateWidget` (`|GetArrayItem` (`self.TextToSpawn`) (`self.CurrentIndex`))))
      (bind _output_get (set `self.SpawnedText` _returnvalue))
      (if (`KismetSystemLibrary.IsValid` _output_get)
        (`UserWidget.AddToViewport` _output_get 0))
      (if (== (`KismetArrayLibrary.Array_Length` (`self.TextToSpawn`)) (+ (`self.CurrentIndex`) 1))
        (set `self.NoMoreText` true)
        (else
          (set `self.CurrentIndex` (+ (`self.CurrentIndex`) 1)))))))

(fn `UserConstructionScript`)